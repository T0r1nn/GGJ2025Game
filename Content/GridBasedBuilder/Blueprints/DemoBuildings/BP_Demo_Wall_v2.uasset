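; BP_Demo_Wall_v2 is a demo placeable wall for the grid-based builder that adapts its shape to surrounding walls.
; BuildManager computes an 8-way part index for its cell and class, which looks up the mesh and yaw in index and angle tables.
; It refreshes on BeginPlay and UpdateFromObject, and calls UpdateNeighborObjects when spawned, demolished or destroyed, so adjacent pieces can follow.
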(event `self.ReceiveBeginPlay`
  (`parent.ReceiveBeginPlay`)
  (bind _partindex (`/Game/GridBasedBuilder/Blueprints/BP_BuildManager.8CalculatePartIndexForObject` (`self.BuildManager`) (`self.OccupiedCenterCell`) (`GameplayStatics.GetObjectClass` self)))
  (set `self.PartIndex` _partindex)
  (`StaticMeshComponent.SetStaticMesh` (`self.StaticMesh`) (`|GetArrayItem` (`self.WallMeshes`) (`|GetArrayItem` (`self.WallIndexes`) (`self.PartIndex`))))
  (`SceneComponent.K2_SetRelativeRotation` (`self.StaticMesh`) (`KismetMathLibrary.MakeRotator` 0.0 0.0 (`|GetArrayItem` (`self.WallAngles`) (`self.PartIndex`))) false false)
  (`self.UpdateNeighborObjects`))

(fn `DemolitionPlaceableObject`
  (params (SideOfRequestOwner :type Integer))
  (`parent.DemolitionPlaceableObject` SideOfRequestOwner)
  (`self.UpdateNeighborObjects`))

(fn `DestroyPlaceableObject`
  (`parent.DestroyPlaceableObject`)
  (`self.UpdateNeighborObjects`))

(fn `UpdateFromObject`
  (params (FromCell :type "IntPoint Structure") (ByObject :type "/Game/GridBasedBuilder/Blueprints/BP_PlaceableObject_Base_Class Object Reference") (ObjectWasSpawned :type Boolean))
  (bind _partindex (`/Game/GridBasedBuilder/Blueprints/BP_BuildManager.8CalculatePartIndexForObject` (`self.BuildManager`) (`self.OccupiedCenterCell`) (`GameplayStatics.GetObjectClass` self)))
  (set `self.PartIndex` _partindex)
  (`StaticMeshComponent.SetStaticMesh` (`self.StaticMesh`) (`|GetArrayItem` (`self.WallMeshes`) (`|GetArrayItem` (`self.WallIndexes`) (`self.PartIndex`))))
  (`SceneComponent.K2_SetRelativeRotation` (`self.StaticMesh`) (`KismetMathLibrary.MakeRotator` 0.0 0.0 (`|GetArrayItem` (`self.WallAngles`) (`self.PartIndex`))) false false))

(fn `UserConstructionScript`)