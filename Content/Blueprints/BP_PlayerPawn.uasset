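; BP_PlayerPawn is a player pawn that acts as a movable camera, panned through Enhanced Input.
; On BeginPlay it rotates its root component by 45 degrees and moves itself to a fixed point raised above the world origin.
; The X and Y camera input actions add swept local offsets scaled by CameraSpeed, so panning follows the rotated axes and is not scaled by frame time.
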(event `self.ReceiveBeginPlay`
  (`SceneComponent.K2_SetWorldRotation` (`self.RootComponent`) (struct :`Yaw` 45.0) false false)
  (`self.K2_SetActorLocation` (0.0 0.0 100.0)))

(event `EnhancedInput|/Game/Blueprints/InputActions/IA_CameraXMovement`
  (params (ActionValue :type "Float (double-precision)") (ElapsedSeconds :type "Float (double-precision)") (TriggeredSeconds :type "Float (double-precision)") (InputAction :type "InputAction Object Reference" :default "/Game/Blueprints/InputActions/IA_CameraXMovement.IA_CameraXMovement"))
  (:`Triggered`
    (`self.K2_AddActorLocalOffset` (`KismetMathLibrary.MakeVector` (* ActionValue (`self.CameraSpeed`))) true)))

(event `EnhancedInput|/Game/Blueprints/InputActions/IA_CameraYMovement`
  (params (ActionValue :type "Float (double-precision)") (ElapsedSeconds :type "Float (double-precision)") (TriggeredSeconds :type "Float (double-precision)") (InputAction :type "InputAction Object Reference" :default "/Game/Blueprints/InputActions/IA_CameraYMovement.IA_CameraYMovement"))
  (:`Triggered`
    (`self.K2_AddActorLocalOffset` (`KismetMathLibrary.MakeVector` 0.0 (* ActionValue (`self.CameraSpeed`))) true)))

(fn `UserConstructionScript`)