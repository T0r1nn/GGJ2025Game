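; BP_Tetromino_Placer is a grid-based build placer, apparently for tetromino pieces, that validates a build area and spawns the placeable object.
; BuildObject forces an indicator refresh through DrawPlacementIndicators, whose graph rechecks CanBuild and any units blocking the area before spawning.
; The spawn centers on the BuildManager's cursor cell, passing table name, cell and direction as dynamic data.
; HighlightBuildingsInArea is empty, and the event graph is inactive.
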(fn `BuildObject`
  (set `self.ForceUpdatePlaceIndicators` true)
  (`self.DrawPlacementIndicators`))

(fn `DrawPlacementIndicators`
  (bind _buildmanager (`self.BuildManager`))
  (bind _cellundercursor (`/Game/GridBasedBuilder/Blueprints/BP_BuildManager.CellUnderCursor` (`self.BuildManager`)))
  (bind (_locationundercursor_camera__x _locationundercursor_camera__y _locationundercursor_camera__z) (`KismetMathLibrary.BreakVector` (`/Game/GridBasedBuilder/Blueprints/BP_BuildManager.LocationUnderCursor(Camera)` _buildmanager)))
  (bind (_center_x _center_y) (`KismetMathLibrary.BreakVector2D` (`/Game/GridBasedBuilder/Blueprints/BP_BuildManager.GetCenterOfRectangularArea` _buildmanager _cellundercursor (`self.ObjectSize`))))
  (set `self.ForceUpdatePlaceIndicators` true)
  (`self.DrawPlacementIndicators`) ; Final check construction area
  (if (and (`self.CanBuild`) (not (and (`self.CheckUnitsInBuildArea`) (`self.HasUnitsInBuildArea`))))
    (set `self.ForceUpdatePlaceIndicators` true)
    (`|SpawnActorFromClass` (`self.PlaceableObjectClass`) (`KismetMathLibrary.MakeTransform` (`KismetMathLibrary.MakeVector` _center_x _center_y _locationundercursor_camera__z)) "Undefined" "SelectDefaultAtRuntime" null (`self.ObjectNameInTable`) (make `/Game/GridBasedBuilder/Data/S_PlaceableObjects_Dynamic_Data` true _buildmanager _cellundercursor (`self.BuildDirection`)) null)))

(fn `HighlightBuildingsInArea`)

(fn `UserConstructionScript`
  (`parent.UserConstructionScript`))