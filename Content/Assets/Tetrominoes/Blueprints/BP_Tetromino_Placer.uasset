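; Placer for tetromino-shaped buildings on the BuildManager grid, extending a parent object placer with multi-cell footprints defined by ObjectOffsets.
; When the hovered cell changes or an update is forced, it moves the preview mesh, checks each cell's occupancy and height, and sets accepted or rejected material.
; Rotation turns the offsets 90 degrees.
; Building rechecks validity, then spawns one single-cell placeable per cell at hardcoded spacing and marks it occupied.
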(event `self.ReceiveBeginPlay`
  (bind (_objectsize_x _objectsize_y) (break `IntPoint` (`self.ObjectSize`)))
  (bind _returnvalue (/ (`/Game/GridBasedBuilder/Blueprints/BP_BuildManager.GridCellSizeXY` (`self.BuildManager`)) 110.0))
  (`parent.ReceiveBeginPlay`) ; Object Data setting here
  (set `self.ForceUpdatePlaceIndicators` true)
  (for _ (range (* _objectsize_x _objectsize_y))
    (bind _staticmesh (`self.GetReusableMesh` (`self.PlaceIndicators`) (`self.PlaceMeshUsingAmount`) "/Game/GridBasedBuilder/Meshes/SM_Plane_100x100.SM_Plane_100x100" true))
    (`SceneComponent.SetRelativeScale3D` _staticmesh (`KismetMathLibrary.MakeVector` _returnvalue _returnvalue 1.0))))

(event `self.ReceiveTick`
  (params (DeltaSeconds :type "Float (single-precision)"))
  (`self.GeneratePlacementData`))

(fn `BuildObject`
  (bind _cellsforbuild (`self.CellsForBuild`))
  (set `self.ForceUpdatePlaceIndicators` true)
  (`self.GeneratePlacementData`) ; Final check construction area
  (if (and (`self.CanBuild`) (not (and (`self.CheckUnitsInBuildArea`) (`self.HasUnitsInBuildArea`))))
    (set `self.ForceUpdatePlaceIndicators` true)
    (for (_array_element _array_index) _cellsforbuild
      (`|SpawnActorFromClass` "/Game/Assets/Tetrominoes/Blueprints/BP_Tetromino_Single_Placeable.BP_Tetromino_Single_Placeable_C" (`KismetMathLibrary.MakeTransform` (`KismetMathLibrary.MakeVector` (* (`KismetMathLibrary.Conv_IntToDouble` (break `IntPoint` _array_element)) 200.0) (* (`KismetMathLibrary.Conv_IntToDouble` (`.Y` (break `IntPoint` _array_element))) 200.0))) "Undefined" "MultiplyWithRoot" null (`self.SingleTetrominoData`) (make `/Game/GridBasedBuilder/Data/S_PlaceableObjects_Dynamic_Data` true (`self.BuildManager`) (make `IntPoint` (break `IntPoint` _array_element) (`.Y` (break `IntPoint` _array_element)))) null)
      (`/Game/GridBasedBuilder/Blueprints/BP_BuildManager.SetOccupancyData` (`self.BuildManager`) (`|GetArrayItem` (`self.CellsForBuild`) _array_index) true))
    (`/Game/GridBasedBuilder/Blueprints/BP_BuildManager.OnObjectBuilt` (`self.BuildManager`) _cellsforbuild (`self.PlaceableObjectClass`))))

(fn `GeneratePlacementData`
  (locals (BaseBuildLevelLOCAL :type "Float (double-precision)") (LocationLOCAL :type "Vector Structure") (IndexLOCAL :type Integer))
  (bind _obectmesh (`self.ObectMesh`))
  (bind _buildmanager (`self.BuildManager`))
  (bind _cellundercursor (`/Game/GridBasedBuilder/Blueprints/BP_BuildManager.CellUnderCursor` _buildmanager))
  (bind _cellundercursor_2 (`/Game/GridBasedBuilder/Blueprints/BP_BuildManager.CellUnderCursor` (`self.BuildManager`)))
  (bind (_center_x _center_y) (`KismetMathLibrary.BreakVector2D` (`/Game/GridBasedBuilder/Blueprints/BP_BuildManager.GetCenterOfRectangularArea` _buildmanager _cellundercursor (`self.ObjectSize`))))
  (`|ExecutionSequence`
    (:`then_0`
      (if (or (`/Game/GridBasedBuilder/Blueprints/BP_BuildManager.CellUnderCursorHasChanged` (`self.BuildManager`)) (`self.ForceUpdatePlaceIndicators`))
        (set `self.ForceUpdatePlaceIndicators` false)
        (set `self.CanBuild` true)
        (bind _location (`/Game/GridBasedBuilder/Blueprints/BP_BuildManager.GetCellLocation` _buildmanager _cellundercursor))
        (set `local.BaseBuildLevelLOCAL` (.z _location))
        (`SceneComponent.K2_SetWorldLocation` (`self.ObectMesh`) (`KismetMathLibrary.MakeVector` _center_x _center_y) false false)
        (set `self.CellsForBuild` (`|MakeArray` _cellundercursor_2))
        (for _array_element (`self.ObjectOffsets`)
          (`KismetArrayLibrary.Array_Add` (`self.CellsForBuild`) (+ _array_element _cellundercursor_2)))
        (for _array_element_2 (`self.CellsForBuild`)
          (bind (_location_2 _success) (`/Game/GridBasedBuilder/Blueprints/BP_BuildManager.GetCellLocation` (`self.BuildManager`) _array_element_2))
          (if (and (not (`/Game/GridBasedBuilder/Blueprints/BP_BuildManager.GetOccupancyData` (`self.BuildManager`) _array_element_2)) _success (< (`KismetMathLibrary.Abs` (- (.z _location_2) (`local.BaseBuildLevelLOCAL`))) (`self.MaxHeightDifferenceForConstruction`)))
            (`PrimitiveComponent.SetMaterial` _obectmesh 0 (`self.PlaceAcceptedMaterial`))
            (else
              (`PrimitiveComponent.SetMaterial` _obectmesh 0 (`self.PlaceRejectedMaterial`))
              (set `self.CanBuild` false)
              (break))))))))

(fn `RotateObjectPlacer`
  (params (Left :type Boolean))
  (`parent.RotateObjectPlacer` Left)
  (for (_array_element _array_index) (`self.ObjectOffsets`)
    (`KismetArrayLibrary.Array_Set` (`self.ObjectOffsets`) _array_index (make `IntPoint` (* (`.Y` (break `IntPoint` _array_element)) -1) (break `IntPoint` _array_element))))
  (set `self.ForceUpdatePlaceIndicators` true))

(fn `SetupObjectPlacer`
  (`parent.SetupObjectPlacer`)
  (`StaticMeshComponent.SetStaticMesh` (`self.ObectMesh`) (`.Mesh_111_372903284934DB726046BDA1ACC6566A` (break `/Game/GridBasedBuilder/Data/S_PlaceableObjects_Data` (`self.ObjectData`)))))

(fn `UserConstructionScript`)