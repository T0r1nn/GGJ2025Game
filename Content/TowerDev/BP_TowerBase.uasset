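; Base tower that fires harpoon-sounding projectiles at Bubble_Blueprint enemies inside its FireRange.
; Overlaps maintain ActorsInRange, and a DoOnce calls StartAutoFire on entry, though that function graph is empty and CustomEvent holds the looping fire timer.
; Each shot retargets by greatest TotalTime, not distance, then spawns a projectile and rotates the turret pivot toward it.
; An empty range stops firing and resets the DoOnce; findclosest is an uncalled leftover.
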(event `self.Fire Range.OnComponentBeginOverlap`
  (params (OverlappedComponent :type "PrimitiveComponent Object Reference") (OtherActor :type "Actor Object Reference") (OtherComp :type "PrimitiveComponent Object Reference") (OtherBodyIndex :type Integer) (bFromSweep :type Boolean) (SweepResult :type "HitResult Structure (by ref)"))
  ; Add all entering actors into array
  (`KismetSystemLibrary.IsObjectOfSoftClass` OtherActor "/Game/Bubbles/Bubble_Blueprint.Bubble_Blueprint_C"
    (:`True`
      (`KismetArrayLibrary.Array_Add` (`self.ActorsInRange`) OtherActor)
      (`/Engine/EditorBlueprintResources/StandardMacros.DoOnce` false :!label _label
        (:`Completed`
          (`self.StartAutoFire`))))))

(event `ResetAutoFireCheck`
  (goto _label :!via `Reset`))

(event `self.ReceiveBeginPlay`
  ; Find first enemy
  (`KismetSystemLibrary.K2_SetTimerDelegate` :`Time` 0.5 :`bLooping` true))

(event `FindNewTarget`
  ; Find first enemy
  (`KismetSystemLibrary.PrintString` (`KismetSystemLibrary.GetDisplayName` (`self.TargetActor`)) true true (struct :`R` 1.0 :`G` 0.814041 :`A` 1.0) 0.5)
  (if (`KismetArrayLibrary.Array_IsNotEmpty` (`self.ActorsInRange`))
    (for _array_element (`self.ActorsInRange`)
      (if (`KismetSystemLibrary.IsValid` (`self.TargetActor`))
        (bind _asbubble_blueprint (cast `/Game/Bubbles/Bubble_Blueprint` _array_element))
        (bind _asbubble_blueprint_2 (cast `/Game/Bubbles/Bubble_Blueprint` (`self.TargetActor`)))
        (if (> (`/Game/Bubbles/Bubble_Blueprint.TotalTime` _asbubble_blueprint) (`/Game/Bubbles/Bubble_Blueprint.TotalTime` _asbubble_blueprint_2))
          (set `self.TargetActor` _array_element))
        (else
          (set `self.TargetActor` _array_element))))))

(event `findclosest`
  ; Find Closest Actor to Tower
  (for (_array_element _array_index) (`self.ActorsInRange`)
    (if (`KismetSystemLibrary.IsValid` (`self.TargetActor`))
      (set `self.TargetActor` _array_element)
      (else
        (`KismetSystemLibrary.IsObjectOfSoftClass` _array_element "/Game/TowerDev/Tower_Enemy.Tower_Enemy_C"
          (:`True`
            (if (< (`self.GetDistanceTo` (`self.TargetActor`)) (`self.GetDistanceTo` _array_element))
              (set `self.TargetActor` _array_element))))))))

(event `self.Fire Range.OnComponentEndOverlap`
  (params (OverlappedComponent :type "PrimitiveComponent Object Reference") (OtherActor :type "Actor Object Reference") (OtherComp :type "PrimitiveComponent Object Reference") (OtherBodyIndex :type Integer))
  ; Spawns projectile. Makes hitboxes and turret look at target.
  (`KismetSystemLibrary.IsObjectOfSoftClass` OtherActor "/Game/Bubbles/Bubble_Blueprint.Bubble_Blueprint_C"
    (:`True`
      (`KismetArrayLibrary.Array_RemoveItem` (`self.ActorsInRange`) OtherActor)
      (`KismetSystemLibrary.PrintString` (`KismetSystemLibrary.GetDisplayName` OtherActor) true true (struct :`R` 1.0 :`B` 0.020533 :`A` 1.0)))))

(event `StopAutoFire`
  ; Spawns projectile. Makes hitboxes and turret look at target.
  (`KismetSystemLibrary.K2_ClearAndInvalidateTimerHandle` (`self.Timer`)))

(event `CustomEvent`
  (bind _firerate (`self.FireRate`))
  ; Spawns projectile. Makes hitboxes and turret look at target.
  (bind _returnvalue (`KismetSystemLibrary.K2_SetTimerDelegate` (delegate `FireProjectile`) _firerate true false (* _firerate -1.0)))
  (set `self.Timer` _returnvalue))

(event `FireProjectile`
  (bind _turretpivot (`self.TurretPivot`))
  (bind _returnvalue (`KismetMathLibrary.TransformLocation` (`SceneComponent.K2_GetComponentToWorld` (`self.ProjectileSpawner`))))
  (bind _returnvalue_2 (`KismetMathLibrary.Conv_VectorToRotator` (`KismetMathLibrary.GetDirectionUnitVector` _returnvalue (`self.K2_GetActorLocation` (`self.TargetActor`)))))
  ; Spawns projectile. Makes hitboxes and turret look at target.
  (`AkGameplayStatics.PostEvent` "/Game/WwiseAudio/TurretHarpoon.TurretHarpoon")
  (if (`KismetArrayLibrary.Array_IsNotEmpty` (`self.ActorsInRange`))
    (`self.FindNewTarget`)
    (bind _asbubble_blueprint (cast `/Game/Bubbles/Bubble_Blueprint` (`self.TargetActor`)))
    (`|SpawnActorFromClass` "/Game/TowerDev/Projectile.Projectile_C" (`KismetMathLibrary.MakeTransform` _returnvalue _returnvalue_2) "Undefined" "OverrideRootScale" self _asbubble_blueprint null)
    (`SceneComponent.K2_SetRelativeRotation` _turretpivot _returnvalue_2 false false)
    (`SceneComponent.K2_AddLocalRotation` _turretpivot (struct :`Yaw` 270.0) false false)
    (else
      (`self.StopAutoFire`)
      (`self.ResetAutoFireCheck`))))

(fn `StartAutoFire`)

(fn `StopAutoFire`)

(fn `UserConstructionScript`)